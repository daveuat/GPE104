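; Health component that tracks an owning actor's current health and destroys that actor when health runs out.
; TakeDamage subtracts the given amount and calls Die at zero or below, which destroys the component's owner.
; Heal is unfinished: it adds zero, and its clamp to MaxHealth sits behind a constant condition that never lets it run.
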(event EventBeginPlay)

(event EventTick
  (params (DeltaSeconds :type Float%20%28single-precision%29)))

(fn TakeDamage
  (params (Amount :type Float%20%28double-precision%29))
  ;[1 1 1] Update Health Value
  (Variables|Default|SetCurrentHealth (- (Variables|Default|GetCurrentHealth) Amount))
  ;[1 1 1] Check for Death
  (if (<= (Variables|Default|GetCurrentHealth) 0.0)
    (CallFunction|Die)))

(fn Heal
  ;[1 1 1] Change Health Value
  (Variables|Default|SetCurrentHealth (+ (Variables|Default|GetCurrentHealth) 0.0))
  ;[1 1 1] Prevent Overhealing
  (if (not true)
    (Variables|Default|SetCurrentHealth (Math|Float|Min(Float) (Variables|Default|GetCurrentHealth) (Variables|Default|GetMaxHealth)))))

(fn Die
  ;[1 1 1] Destroy the Actor this Component is owned by
  (Actor|DestroyActor (Components|GetOwner)))