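; EnemySphere is an enemy actor that chases the player and explodes on contact.
; While chasing is enabled, Tick moves it toward the player pawn with a swept, speed-scaled step; otherwise it prints a not-moving message.
; Hit and overlap run duplicate chains: deal fixed damage, spawn an actor at its transform, destroy itself, call DestroyActor on the player controller, and print a damage message.
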(event Collision|EventActorBeginOverlap
  (params (OtherActor :type Actor%20Object%20Reference))
  ;[1 1 1] Damage Overlapping Actor
  (Game|Damage|ApplyDamage OtherActor 2e+01 0 0)
  ;[1 1 1] Explode
  (Game|SpawnActorfromClass "/Game/StarterContent/Blueprints/Blueprint_Effect_Explosion.Blueprint_Effect_Explosion_C" (Transformation|GetActorTransform) "Undefined" 0 0)
  (Actor|DestroyActor)
  (Actor|DestroyActor (Game|GetPlayerController 0))
  (Development|PrintText "You took 20 damage."))

(event EventTick
  (params (DeltaSeconds :type Float%20%28single-precision%29))
  ;[1 1 1] Object move and vector to player
  (if (Variables|Default|GetisChasingPlayer)
    (Transformation|SetActorLocation (+ (Transformation|GetActorLocation) (* (Math|Vector|Normalize (- (Transformation|GetActorLocation (Game|Player|GetPlayerPawn 0)) (Transformation|GetActorLocation))) (* (Variables|Default|GetSpeed) DeltaSeconds))) true false)
    (else
      (Development|PrintString (Variables|Default|GetNotMovingText)))))

(event Collision|EventHit
  (params (MyComp :type Primitive%20Component%20Object%20Reference) (Other :type Actor%20Object%20Reference) (OtherComp :type Primitive%20Component%20Object%20Reference) (bSelfMoved :type Boolean) (HitLocation :type Vector :default "0, 0, 0") (HitNormal :type Vector :default "0, 0, 0") (NormalImpulse :type Vector :default "0, 0, 0") (Hit :type Hit%20Result%20Structure%20%28by%20ref%29))
  ;[1 1 1] Events When Hit Or Touch
  (Game|Damage|ApplyDamage Other 2e+01 0 0)
  (Game|SpawnActorfromClass "/Game/StarterContent/Blueprints/Blueprint_Effect_Explosion.Blueprint_Effect_Explosion_C" (Transformation|GetActorTransform) "Undefined" 0 0)
  (Actor|DestroyActor)
  (Actor|DestroyActor (Game|GetPlayerController 0))
  (Development|PrintText "You took 20 damage."))

(fn ConstructionScript)